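; BP_Warpcore is a warp core scene item whose Niagara particle effect can be made denser or sparser.
; AddParticles and RemoveParticles raise or lower ParticleCount by a fixed step, write it to the Niagara UserSpawnRate variable, and return the new value.
; The count is not clamped, and the event graph holds no active logic, so changes happen only when these functions are called.
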(fn `AddParticles`
  (returns (NewParam :type "Float (double-precision)"))
  (bind _output_get (set `self.ParticleCount` (+ (`self.ParticleCount`) 500.0)))
  (`NiagaraComponent.SetVariableFloat` (`self.Niagara`) "UserSpawnRate" _output_get)
  (return (`self.ParticleCount`)))

(fn `RemoveParticles`
  (returns (NewParam :type "Float (double-precision)"))
  (bind _output_get (set `self.ParticleCount` (- (`self.ParticleCount`) 500.0)))
  (`NiagaraComponent.SetVariableFloat` (`self.Niagara`) "UserSpawnRate" _output_get)
  (return (`self.ParticleCount`)))

(fn `UserConstructionScript`)