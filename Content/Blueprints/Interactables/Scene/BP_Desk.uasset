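; BP_Desk is an interactable desk with a drawer that toggles open and closed on interaction.
; Its InteractLogic override ignores the toggle while animating, otherwise fires OpenDrawer or CloseDrawer, and always calls the parent logic afterwards.
; Each event plays its own sound and timeline, lerping the drawer mesh along relative Y, then updates the closed and animating flags on finish.
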(event `OpenDrawer`
  (bind _audio (`self.Audio`))
  (bind _staticmesh3 (`self.StaticMesh3`))
  (bind (_relativelocation_x _relativelocation_y _relativelocation_z) (`KismetMathLibrary.BreakVector` (`SceneComponent.RelativeLocation` _staticmesh3)))
  (`AudioComponent.SetSound` _audio "/Game/SFX/DrawerOpen_BW_14092.DrawerOpen_BW_14092")
  (`AudioComponent.Play` _audio 0.0)
  (set `self.isAnimating` true)
  (bind (_direction _newtrack_0) (`Timeline|Timeline_0` :!via `PlayFromStart`)
    (:`Update`
      (`SceneComponent.K2_SetRelativeLocation` _staticmesh3 (`KismetMathLibrary.MakeVector` _relativelocation_x (`KismetMathLibrary.Lerp` (`self.InitialPosition`) (`self.OpenPosition`) _newtrack_0) _relativelocation_z) false false))
    (:`Finished`
      (set `self.DrawerClosed` false)
      (set `self.isAnimating` false))))

(event `CloseDrawer`
  (bind _audio (`self.Audio`))
  (bind _staticmesh3 (`self.StaticMesh3`))
  (bind (_relativelocation_x _relativelocation_y _relativelocation_z) (`KismetMathLibrary.BreakVector` (`SceneComponent.RelativeLocation` _staticmesh3)))
  (`AudioComponent.SetSound` _audio "/Game/SFX/DrawerClose_BW_13982.DrawerClose_BW_13982")
  (`AudioComponent.Play` _audio 0.0)
  (set `self.isAnimating` true)
  (bind (_direction _newtrack_0) (`Timeline|Timeline_1` :!via `PlayFromStart`)
    (:`Update`
      (`SceneComponent.K2_SetRelativeLocation` _staticmesh3 (`KismetMathLibrary.MakeVector` _relativelocation_x (`KismetMathLibrary.Lerp` (`self.InitialPosition`) (`self.OpenPosition`) _newtrack_0) _relativelocation_z) false false))
    (:`Finished`
      (set `self.DrawerClosed` true)
      (set `self.isAnimating` false))))

(fn `InteractLogic`
  (if (`self.isAnimating`)
    _
    (elif (`self.DrawerClosed`)
      (`self.OpenDrawer`)
      (else
        (`self.CloseDrawer`))))
  (`parent.InteractLogic`))

(fn `UserConstructionScript`
  (`parent.UserConstructionScript`))