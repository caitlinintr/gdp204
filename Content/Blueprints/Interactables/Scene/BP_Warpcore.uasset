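; Interactable warp core that showcases a Niagara effect, switchable between CPU and GPU simulation.
; Interact swaps the Niagara asset and updates the processor label, while add and remove events step the particle count and refresh its readout.
; A box trigger shows both text labels while the first-person character is inside.
; The Fixed event lowers the audio volume and drives the effect's fix progress through a timeline.
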(event `self.ReceiveBeginPlay`
  (set `self.NiagaraSytemVFX` (`NiagaraComponent.GetAsset` (`self.Niagara`))))

(event `Fixed`
  (`AudioComponent.AdjustVolume` (`self.Audio`) 3.0 0.2 "Sin")
  (bind (_direction _newtrack_0) (`Timeline|Timeline_0` :!via `PlayFromStart`)
    (:`Update`
      (`FXSystemComponent.SetFloatParameter` (`self.Niagara`) "User.fixProgress" _newtrack_0))))

(event `self.Box.OnComponentBeginOverlap`
  (params (OverlappedComponent :type "PrimitiveComponent Object Reference") (OtherActor :type "Actor Object Reference") (OtherComp :type "PrimitiveComponent Object Reference") (OtherBodyIndex :type Integer) (bFromSweep :type Boolean) (SweepResult :type "HitResult Structure (by ref)"))
  (cast `/Game/FirstPerson/Blueprints/BP_FirstPersonCharacter` OtherActor)
  (`SceneComponent.SetVisibility` (`self.Text_Processor`) true false)
  (`SceneComponent.SetVisibility` (`self.Text_ParticleCount`) true false))

(event `self.Box.OnComponentEndOverlap`
  (params (OverlappedComponent :type "PrimitiveComponent Object Reference") (OtherActor :type "Actor Object Reference") (OtherComp :type "PrimitiveComponent Object Reference") (OtherBodyIndex :type Integer))
  (cast `/Game/FirstPerson/Blueprints/BP_FirstPersonCharacter` OtherActor)
  (`SceneComponent.SetVisibility` (`self.Text_Processor`) false true)
  (`SceneComponent.SetVisibility` (`self.Text_ParticleCount`) false true))

(event `/Game/Blueprints/Interfaces/I_Interactable.Interact`
  (params (Character :type "/Game/FirstPerson/Blueprints/BP_FirstPersonCharacter Object Reference"))
  (bind _niagarasystemgpu (`self.NiagaraSystemGPU`))
  (bind _text_processor (`self.Text_Processor`))
  (bind _niagara (`self.Niagara`))
  (bind _niagara_2 (`self.Niagara`))
  (bind _niagarasystemcpu (`self.NiagaraSystemCPU`))
  (if (`self.IsCPU`)
    (`NiagaraComponent.SetAsset` _niagara_2 _niagarasystemgpu true)
    (set `self.NiagaraSytemVFX` _niagarasystemgpu)
    (set `self.IsCPU` false)
    (`NiagaraComponent.SetVariableFloat` _niagara "UserSpawnRate" (`self.Particle Count`))
    (`TextRenderComponent.K2_SetText` _text_processor (`self.GPU TEXT`))
    (else
      (`NiagaraComponent.SetAsset` _niagara_2 _niagarasystemcpu true)
      (set `self.NiagaraSytemVFX` _niagarasystemcpu)
      (set `self.IsCPU` true)
      (`NiagaraComponent.SetVariableFloat` _niagara "UserSpawnRate" (`self.Particle Count`))
      (`TextRenderComponent.K2_SetText` _text_processor (`self.CPU TEXT`)))))

(event `OnAddParticles`
  (`self.AddParticles`)
  (`TextRenderComponent.K2_SetText` (`self.Text_ParticleCount`) (`|FormatText` "Particles: {Count}" (`self.Particle Count`)) :!label _label))

(event `OnRemoveParticles`
  (`self.RemoveParticles`)
  (goto _label))

(fn `AddParticles`
  (returns (NewParam :type "Float (double-precision)"))
  (bind _output_get (set `self.Particle Count` (+ (`self.Particle Count`) 500.0)))
  (`NiagaraComponent.SetVariableFloat` (`self.Niagara`) "User.particleCount" _output_get)
  (return (`self.Particle Count`)))

(fn `RemoveParticles`
  (returns (NewParam :type "Float (double-precision)"))
  (if (> (`self.Particle Count`) 0.0)
    (bind _output_get (set `self.Particle Count` (- (`self.Particle Count`) 500.0)))
    (`NiagaraComponent.SetVariableFloat` (`self.Niagara`) "User.particleCount" _output_get)
    (return (`self.Particle Count`))))

(fn `UserConstructionScript`
  (`TextRenderComponent.K2_SetText` (`self.Text_Processor`) (`self.CPU TEXT`))
  (`TextRenderComponent.K2_SetText` (`self.Text_ParticleCount`) (`|FormatText` "Particles: {count}" (`self.Particle Count`))))