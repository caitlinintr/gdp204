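; Interactable puzzle lever that toggles between up and down states, exposing its status to an assigned puzzle.
; InteractLogic ignores toggling while animating, otherwise calls PushLever or ReleaseLever, then always runs the parent logic.
; Each direction plays its own sound and a timeline that lerps the lever's roll between initial and final rotations.
; When a timeline finishes, it updates LeverUp and tells the puzzle to check for a correct solution.
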(event `PushLever`
  (bind _audio (`self.Audio`))
  (`AudioComponent.SetSound` _audio "/Game/SFX/PneumaticLever_jwEvH_11.PneumaticLever_jwEvH_11")
  (`AudioComponent.Play` _audio 0.0)
  (set `self.isAnimating` true)
  (bind (_direction _newtrack_0) (`Timeline|Timeline_0` :!via `PlayFromStart`)
    (:`Update`
      (`SceneComponent.K2_SetRelativeRotation` (`self.Lever`) (`KismetMathLibrary.MakeRotator` (`KismetMathLibrary.Lerp` (`self.InitialRotation`) (`self.Final Rotation`) _newtrack_0)) false false))
    (:`Finished`
      (set `self.LeverUp` false)
      (set `self.isAnimating` false)
      (`/Game/Blueprints/Puzzles/BP_PuzzleBase.CheckIfPuzzleCorrect` (`self.Puzzle`)))))

(event `ReleaseLever`
  (bind _audio (`self.Audio`))
  (`AudioComponent.SetSound` _audio "/Game/SFX/LeverHinge_BW_9219.LeverHinge_BW_9219")
  (`AudioComponent.Play` _audio 0.0)
  (set `self.isAnimating` true)
  (bind (_direction _newtrack_0) (`Timeline|Timeline_1` :!via `PlayFromStart`)
    (:`Update`
      (`SceneComponent.K2_SetRelativeRotation` (`self.Lever`) (`KismetMathLibrary.MakeRotator` (`KismetMathLibrary.Lerp` (`self.InitialRotation`) (`self.Final Rotation`) _newtrack_0)) false false))
    (:`Finished`
      (set `self.LeverUp` true)
      (set `self.isAnimating` false)
      (`/Game/Blueprints/Puzzles/BP_PuzzleBase.CheckIfPuzzleCorrect` (`self.Puzzle`)))))

(event `/Game/Blueprints/Interfaces/I_PuzzlePiece.AssignPuzzle`
  (params (Puzzle :type "/Game/Blueprints/Puzzles/BP_PuzzleBase Object Reference"))
  (set `self.Puzzle` Puzzle))

(fn `GetStatus`
  (returns (PieceStatus :type Boolean))
  (return (`self.LeverUp`)))

(fn `InteractLogic`
  (if (`self.isAnimating`)
    _
    (elif (`self.LeverUp`)
      (`self.PushLever`)
      (else
        (`self.ReleaseLever`))))
  (`parent.InteractLogic`))

(fn `UserConstructionScript`
  (`parent.UserConstructionScript`))