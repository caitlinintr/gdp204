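; An interactable keypad button for puzzles that toggles between pressed and released when used, playing a sound on each interaction.
; Both toggle directions update the pressed state and send the button's number to the keypad.
; Button number 11 acts as the submit key, asking the assigned puzzle to check its solution instead of changing state.
; The pressed state is exposed through GetStatus.
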(event `SelectButton`
  (if (== (`self.ButtonNumber`) 11)
    (`KismetSystemLibrary.PrintString` "CheckPuzzle")
    (`/Game/Blueprints/Puzzles/BP_PuzzleBase.CheckIfPuzzleCorrect` (`self.Puzzle`))
    (else
      (`KismetSystemLibrary.PrintString` "Selecting Button")
      (set `self.isPressed` true)
      (`/Game/Blueprints/Interactables/PuzzlePieces/BP_Keypad.PressButton` (`self.Keypad`) (`self.ButtonNumber`)))))

(event `DeselectButton`
  (`KismetSystemLibrary.PrintString` "Deelecting Button")
  (set `self.isPressed` false)
  (`/Game/Blueprints/Interactables/PuzzlePieces/BP_Keypad.PressButton` (`self.Keypad`) (`self.ButtonNumber`)))

(event `/Game/Blueprints/Interfaces/I_PuzzlePiece.AssignPuzzle`
  (params (Puzzle :type "/Game/Blueprints/Puzzles/BP_PuzzleBase Object Reference"))
  (set `self.Puzzle` Puzzle))

(fn `GetStatus`
  (returns (PieceStatus :type Boolean))
  (return (`self.isPressed`)))

(fn `InteractLogic`
  (`AudioComponent.Play` (`self.Audio`) 0.0)
  (if (`self.isPressed`)
    (`self.DeselectButton`)
    (else
      (`self.SelectButton`)))
  (`parent.InteractLogic`))

(fn `UserConstructionScript`
  (`parent.UserConstructionScript`))