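; Interactable table with a drawer that slides open or closed when interacted with.
; The InteractLogic override toggles between OpenDrawer and CloseDrawer based on DrawerClosed, then calls the parent logic.
; Each event runs its own timeline, lerping the drawer's relative Y between InitialPosition and OpenPosition.
; IsAnimating blocks new toggles during movement, and DrawerClosed updates when the timeline finishes.
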(event `OpenDrawer`
  (bind _drawer (`self.Drawer`))
  (bind (_relativelocation_x _relativelocation_y _relativelocation_z) (`KismetMathLibrary.BreakVector` (`SceneComponent.RelativeLocation` _drawer)))
  (set `self.isAnimating` true)
  (bind (_direction _alpha) (`Timeline|Timeline` :!via `PlayFromStart`)
    (:`Update`
      (`SceneComponent.K2_SetRelativeLocation` _drawer (`KismetMathLibrary.MakeVector` _relativelocation_x (`KismetMathLibrary.Lerp` (`self.InitialPosition`) (`self.OpenPosition`) _alpha) _relativelocation_z) false false))
    (:`Finished`
      (set `self.DrawerClosed` false)
      (set `self.isAnimating` false))))

(event `CloseDrawer`
  (bind _drawer (`self.Drawer`))
  (bind (_relativelocation_x _relativelocation_y _relativelocation_z) (`KismetMathLibrary.BreakVector` (`SceneComponent.RelativeLocation` _drawer)))
  (set `self.isAnimating` true)
  (bind (_direction _alpha) (`Timeline|Timeline_0` :!via `PlayFromStart`)
    (:`Update`
      (`SceneComponent.K2_SetRelativeLocation` _drawer (`KismetMathLibrary.MakeVector` _relativelocation_x (`KismetMathLibrary.Lerp` (`self.OpenPosition`) (`self.InitialPosition`) _alpha) _relativelocation_z) false false))
    (:`Finished`
      (set `self.DrawerClosed` true)
      (set `self.isAnimating` false))))

(fn `InteractLogic`
  (if (`self.isAnimating`)
    _
    (elif (`self.DrawerClosed`)
      (`self.OpenDrawer`)
      (else
        (`self.CloseDrawer`))))
  (`parent.InteractLogic`))

(fn `UserConstructionScript`
  (`parent.UserConstructionScript`))