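; A test interactable button that increases or decreases particles on a referenced warp object, depending on its IsAddParticles flag.
; Interact calls the matching add or remove function on that object, then replays the Pressed timeline, which animates the static mesh's X scale as press feedback.
; The construction script labels the text render "Increase Particles" or "Decrease Particles" from the same flag.
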(event `/Game/Blueprints/Interfaces/I_Interactable.Interact`
  (params (Character :type "/Game/FirstPerson/Blueprints/BP_FirstPersonCharacter Object Reference"))
  (bind _warp_object (`self.WArp Object`))
  (if (`self.isAddParticles`)
    (`/Game/Blueprints/Interactables/Scene/BP_Warpcore.OnAddParticles` _warp_object)
    (bind (_direction _newtrack_0) (`Timeline|Pressed` :!via `PlayFromStart` :!label _label)
      (:`Update`
        (`SceneComponent.SetRelativeScale3D` (`self.StaticMesh`) (`KismetMathLibrary.MakeVector` _newtrack_0 1.0 1.0))))
    (else
      (`/Game/Blueprints/Interactables/Scene/BP_Warpcore.OnRemoveParticles` _warp_object)
      (goto _label :!via `PlayFromStart`))))

(fn `UserConstructionScript`
  (bind _textrender (`self.TextRender`))
  (`parent.UserConstructionScript`)
  (if (`self.isAddParticles`)
    (`TextRenderComponent.K2_SetText` _textrender (`|FormatText` "Increase \nParticles"))
    (else
      (`TextRenderComponent.K2_SetText` _textrender (`|FormatText` "Decrease  \nParticles")))))