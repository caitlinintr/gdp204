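; BP_Door is a lockable two-panel sliding door that reacts to overlaps on a trigger box.
; Unlock, and construction if already unlocked, turn the indicator green.
; Overlap begin and end call OpenDoor and CloseDoor, which play sounds and run a timeline lerping both panels' relative positions.
; CloseDoor also passes true to AnimateDoor, leaving the reverse branch unused, and IsAnimating is never set true here.
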(event `Unlock`
  (if (`self.Locked`)
    (set `self.Locked` false)
    (`PrimitiveComponent.SetMaterial` (`self.Indicator`) 0 "/Game/Materials/M_GreenEmissive.M_GreenEmissive")))

(event `self.Box1.OnComponentBeginOverlap`
  (params (OverlappedComponent :type "PrimitiveComponent Object Reference") (OtherActor :type "Actor Object Reference") (OtherComp :type "PrimitiveComponent Object Reference") (OtherBodyIndex :type Integer) (bFromSweep :type Boolean) (SweepResult :type "HitResult Structure (by ref)"))
  (if (`self.Locked`)
    _
    (elif (`self.isOpen`)
      _
      (elif (not (`self.isAnimating`))
        (`self.OpenDoor`)))))

(event `self.Box1.OnComponentEndOverlap`
  (params (OverlappedComponent :type "PrimitiveComponent Object Reference") (OtherActor :type "Actor Object Reference") (OtherComp :type "PrimitiveComponent Object Reference") (OtherBodyIndex :type Integer))
  (if (`self.Locked`)
    _
    (elif (`self.isOpen`)
      (if (not (`self.isAnimating`))
        (`self.CloseDoor`)))))

(event `AnimateDoor`
  (params (Open :type Boolean))
  (if Open
    (bind (_direction _newtrack_0) (`Timeline|Timeline_0` :!via `PlayFromStart` :!label _label)
      (:`Update`
        (`|ExecutionSequence`
          (:`then_0`
            (bind _returnvalue (`KismetMathLibrary.Lerp` 0.0 -30.0 _newtrack_0))
            (`SceneComponent.K2_SetRelativeLocation` (`self.DoorBottom`) (`KismetMathLibrary.MakeVector` (`KismetMathLibrary.Lerp` (`self.InitialPosition`) (`self.OpenPositionBottom`) _newtrack_0) _returnvalue) false false))
          (:`then_1`
            (`SceneComponent.K2_SetRelativeLocation` (`self.DoorTop`) (`KismetMathLibrary.MakeVector` (`KismetMathLibrary.Lerp` (`self.InitialPosition`) (`self.OpenPositionTop`) _newtrack_0) _returnvalue) false false))))
      (:`Finished`
        (set `self.isAnimating` false)))
    (else
      (goto _label :!via `ReverseFromEnd`))))

(fn `CloseDoor`
  (bind _audio (`self.Audio`))
  (`AudioComponent.SetSound` _audio "/Game/SFX/Sci-Fi_Doorway_03.Sci-Fi_Doorway_03")
  (`AudioComponent.Play` _audio 0.0)
  (`self.AnimateDoor` true)
  (set `self.isOpen` false)
  (return))

(fn `OpenDoor`
  (bind _audio (`self.Audio`))
  (`AudioComponent.SetSound` _audio "/Game/SFX/Space_Door_Close_03.Space_Door_Close_03")
  (`AudioComponent.Play` _audio 0.0)
  (`self.AnimateDoor` true)
  (set `self.isOpen` true)
  (return))

(fn `UserConstructionScript`
  (if (not (`self.Locked`))
    (`PrimitiveComponent.SetMaterial` (`self.Indicator`) 0 "/Game/Materials/M_GreenEmissive.M_GreenEmissive")))