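; BP_ElectricFence is an electric fence prop that damages the first-person character when it begins overlapping the collision box.
; On BeginPlay it gives its Plane a dynamic material instance so the field's opacity can be animated.
; A TurnOff event, guarded to run only once, drives that opacity through a timeline and destroys the actor when finished.
; Debug strings print on overlap and shutdown.
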(event `self.ReceiveBeginPlay`
  (bind _plane (`self.Plane`))
  (bind _returnvalue (`PrimitiveComponent.CreateDynamicMaterialInstance` _plane 0 (`PrimitiveComponent.GetMaterial` _plane 0) "None"))
  (set `self.Electric Material` _returnvalue)
  (`PrimitiveComponent.SetMaterial` (`self.Plane`) 0 (`self.Electric Material`)))

(event `TurnOff`
  (if (not (`self.turningoff`))
    (set `self.turningoff` true)
    (`KismetSystemLibrary.PrintString` "Hello")
    (bind (_direction _newtrack_0) (`Timeline|Timeline_0` :!via `PlayFromStart`)
      (:`Update`
        (`MaterialInstanceDynamic.SetScalarParameterValue` (`self.Electric Material`) "Opacity" _newtrack_0))
      (:`Finished`
        (`self.K2_DestroyActor`)))))

(event `self.Collision Box.OnComponentBeginOverlap`
  (params (OverlappedComponent :type "PrimitiveComponent Object Reference") (OtherActor :type "Actor Object Reference") (OtherComp :type "PrimitiveComponent Object Reference") (OtherBodyIndex :type Integer) (bFromSweep :type Boolean) (SweepResult :type "HitResult Structure (by ref)"))
  (bind _asbp_first_person_character (cast `/Game/FirstPerson/Blueprints/BP_FirstPersonCharacter` OtherActor)
    (:`then`
      (`KismetSystemLibrary.PrintString` "Electric Field Overlap")
      (`/Game/FirstPerson/Blueprints/BP_FirstPersonCharacter.onTakeDamange` _asbp_first_person_character 10.0))
    (:`CastFailed`
      (`KismetSystemLibrary.PrintString` "Overlap not character"))))

(fn `UserConstructionScript`)