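; Interactable lever actor that toggles between up and down positions when used.
; Its InteractLogic override picks PushLever or ReleaseLever from the LeverUp state, ignores toggles while IsAnimating, and always calls the parent logic.
; Each event plays a timeline that lerps the mesh's pitch between initial and final rotations, flipping LeverUp and clearing the animation lock when finished.
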(event `PushLever`
  (set `self.isAnimating` true)
  (bind (_direction _alpha) (`Timeline|Timeline` :!via `PlayFromStart`)
    (:`Update`
      (`SceneComponent.K2_SetRelativeRotation` (`self.StaticMesh`) (`KismetMathLibrary.MakeRotator` 0.0 (`KismetMathLibrary.Lerp` (`self.InitialRotation`) (`self.FinalRotation`) _alpha)) false false))
    (:`Finished`
      (set `self.LeverUp` false)
      (set `self.isAnimating` false))))

(event `ReleaseLever`
  (set `self.isAnimating` true)
  (bind (_direction _alpha) (`Timeline|Timeline_0` :!via `PlayFromStart`)
    (:`Update`
      (`SceneComponent.K2_SetRelativeRotation` (`self.StaticMesh`) (`KismetMathLibrary.MakeRotator` 0.0 (`KismetMathLibrary.Lerp` (`self.FinalRotation`) (`self.InitialRotation`) _alpha)) false false))
    (:`Finished`
      (set `self.LeverUp` true)
      (set `self.isAnimating` false))))

(fn `InteractLogic`
  (if (`self.isAnimating`)
    _
    (elif (`self.LeverUp`)
      (`self.PushLever`)
      (else
        (`self.ReleaseLever`))))
  (`parent.InteractLogic`))

(fn `UserConstructionScript`
  (`parent.UserConstructionScript`))