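; BP_PuzzleBase is a puzzle controller base that checks whether linked pieces match a required combination.
; On BeginPlay it takes the PuzzleCombination map's keys as pieces and passes itself to those implementing I_PuzzlePiece.
; CheckIfPuzzleCorrect compares each piece's status to its mapped value, stopping at the first mismatch.
; The branch calling the empty Win and Fail functions is unconnected, so the result only sets IsWinning.
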(event `self.ReceiveBeginPlay`
  (bind _keys (`BlueprintMapLibrary.Map_Keys` (`self.Puzzle Combination`)))
  (set `self.Puzzles` _keys)
  (for _array_element (`self.Puzzles`)
    (if (`KismetSystemLibrary.DoesImplementInterface` _array_element "/Game/Blueprints/Interfaces/I_PuzzlePiece.I_PuzzlePiece_C")
      (message `/Game/Blueprints/Interfaces/I_PuzzlePiece.AssignPuzzle` _array_element self))))

(event `CheckIfPuzzleCorrect`
  (set `self.isWinning` true)
  (for _array_element (`self.Puzzles`)
    (bind _piecestatus (message `/Game/Blueprints/Interfaces/I_PuzzlePiece.GetStatus` _array_element))
    (bind _returnvalue (== _piecestatus (`BlueprintMapLibrary.Map_Find` (`self.Puzzle Combination`) _array_element)))
    (`KismetSystemLibrary.PrintString` (`KismetStringLibrary.Conv_BoolToString` _returnvalue))
    (set `self.isWinning` _returnvalue)
    (if (not (`self.isWinning`))
      (break))))

(fn `Fail`)

(fn `UserConstructionScript`)

(fn `Win`)